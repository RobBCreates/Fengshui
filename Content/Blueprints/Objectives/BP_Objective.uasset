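; BP_Objective is a grid-snapped objective that scores its linked interactable object from 0 to 100 for one of two players.
; On BeginPlay it links the first BP_InteractableBase with a matching object type, or prints an error.
; A looping one-second timer scores either the interactable's on/off state or its proximity within a radius, falling off linearly.
; Each update pushes score and player side to the interactable's material.
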(event `self.ReceiveBeginPlay`
  (`|ExecutionSequence`
    (:`then_0`
      (`|ExecutionSequence`
        (:`then_0`
          (bind _returnvalue (`GameplayStatics.GetActorOfClass` "/Game/Blueprints/Grid/BP_GridManager.BP_GridManager_C"))
          (bind _output_get (set `self.GridManagerRef` _returnvalue))
          (`/Game/Blueprints/Grid/BP_GridManager.SnapToGrid` _output_get self))
        (:`then_1`
          (bind _returnvalue_2 (`GameplayStatics.GetActorOfClass` "/Game/Blueprints/Objectives/BP_ObjectiveManager.BP_ObjectiveManager_C"))
          (set `self.ObjectiveManagerRef` _returnvalue_2)
          (bind _outactors (`GameplayStatics.GetAllActorsOfClass` "/Game/Blueprints/Interactable/BP_InteractableBase.BP_InteractableBase_C"))
          (for _array_element _outactors
            (if (`|EnumEquality` (`/Game/Blueprints/Interactable/BP_InteractableBase.ObjectType` _array_element) (`self.ObjectiveObjectType`))
              (set `self.ObjectiveReference` _array_element)
              (break))))))
    (:`then_1`
      (bind _objectivereference (`self.ObjectiveReference`)
        (:`then`
          (`KismetSystemLibrary.K2_SetTimer` null "UpdateObjectiveScore" 1.0 true))
        (:`else`
          (`KismetSystemLibrary.PrintString` (`KismetStringLibrary.Concat_StrStr` "Objective not connected to: " (`KismetSystemLibrary.GetDisplayName` _objectivereference)) true true (struct :`R` 1.0 :`G` 0.049562 :`A` 1.0) 20.0))))))

(fn `CalculateDistanceFromObjective`
  (returns (WithinThreshold :type Boolean) (DistanceFromObjective :type "Float (double-precision)"))
  (`self.ObjectiveReference`
    (:`then`
      (bind _output_get (set `self.DistanceFromObjective` (`self.GetDistanceTo` (`self.ObjectiveReference`))))
      (return (<= _output_get (`self.ObjectiveRadius`)) _output_get))
    (:`else`)))

(fn `ObjectHasBeenInteracted`
  (if (`self.bIsInteractBasedObjective`)
    (set `self.ObjectiveScore` (`KismetMathLibrary.SelectFloat` 100.0 0.0 (== (`/Game/Blueprints/Interactable/BP_InteractableBase.bIsOn` (`self.ObjectiveReference`)) (`self.ObjectiveIsToTurnOn`))))))

(fn `UpdateObjectiveScore`
  (locals (l_WithinThreshold :type Boolean :default false))
  (bind _withinthreshold (`self.CalculateDistanceFromObjective`))
  (if (`self.bIsInteractBasedObjective`)
    (`self.ObjectHasBeenInteracted`)
    (`/Game/Blueprints/Interactable/BP_InteractableBase.UpdateMaterial` (`self.ObjectiveReference`) (`self.bIsPlayer2Objective`) (`self.ObjectiveScore`) true)
    (else
      (set `local.l_WithinThreshold` _withinthreshold)
      (if _withinthreshold
        (set `self.ObjectiveScore` (* (- 1.0 (/ (`self.DistanceFromObjective`) (`self.ObjectiveRadius`))) 100.0))
        (else
          (set `self.ObjectiveScore` 0.0)))
      (`/Game/Blueprints/Interactable/BP_InteractableBase.UpdateMaterial` (`self.ObjectiveReference`) (`self.bIsPlayer2Objective`) (/ (`self.ObjectiveScore`) 100.0) (`local.l_WithinThreshold`)))))

(fn `UserConstructionScript`)