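; SceneComp_Movement is a scene component that handles grid-based movement for its owning actor.
; On BeginPlay it caches BP_GridManager, and Move asks it whether the node one fixed step away is free.
; A free node updates the manager, stores the target position and flags Moving; a blocked one calls PushObject, which is an empty stub.
; The lerp, delays and grid-point update are unwired, so the actor never actually moves here.
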(event `self.ReceiveBeginPlay`
  (bind _returnvalue (`GameplayStatics.GetActorOfClass` "/Game/Blueprints/Grid/BP_GridManager.BP_GridManager_C"))
  (set `self.GridManager` _returnvalue))

(event `Move`
  (params (CurrentDirection :type "Vector Structure"))
  (bind _returnvalue (* (`self.CurrentDirection`) 100.0))
  (`self.GridManager`
    (:`then`
      (set `self.CurrentDirection` CurrentDirection)
      (set `self.StartLocation` (`Actor.K2_GetActorLocation` (`self.GetOwner`)))
      (bind (_isspaceavailable _newgridlocation) (`/Game/Blueprints/Grid/BP_GridManager.IsNodeAvailable` (`self.GridManager`) (`self.CurrentGridPoint`) _returnvalue))
      (if _isspaceavailable
        (`/Game/Blueprints/Grid/BP_GridManager.UpdateLocation` (`self.GridManager`) (`self.CurrentGridPoint`) _newgridlocation)
        (set `self.NewPosition` (+ (`self.StartLocation`) _returnvalue))
        (set `self.bMoving` true)
        (else
          (`self.PushObject` _newgridlocation))))
    (:`else`)))

(fn `PushObject`
  (params (GridPointOfInteractable :type "/Game/Blueprints/Grid/BP_GridPoint Object Reference")))