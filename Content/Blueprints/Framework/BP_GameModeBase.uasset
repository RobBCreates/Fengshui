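; Base game mode that sets up a two-player local game with a shared camera and tracks the current game state.
; On BeginPlay, Init resets the state and caches the level's BP_Camera.
; SpawnPlayers then creates local players, spawns a BP_Character for each spaced along Y, possesses it and points both controllers at that camera.
; Getter and setter functions expose the state enum, and StartGame switches it with a debug print.
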(event `self.ReceiveBeginPlay`
  (`self.Init`)
  (`self.SpawnPlayers`))

(fn `GetGameState`
  (returns (CurrentState :type "/Game/Blueprints/Framework/EGameState Enum"))
  (return (`self.CurrentGameState`)))

(fn `Init`
  (set `self.CurrentGameState` "NewEnumerator0")
  (bind _returnvalue (`GameplayStatics.GetActorOfClass` "/Game/Blueprints/Framework/BP_Camera.BP_Camera_C"))
  (set `self.CameraRef` _returnvalue))

(fn `SetGameState`
  (params (NewState :type "/Game/Blueprints/Framework/EGameState Enum" :default "NewEnumerator0"))
  (returns (Return :type Boolean))
  (set `self.CurrentGameState` NewState)
  (return false))

(fn `SpawnPlayers`
  (bind _returnvalue (`GameplayStatics.GetPlayerController` (`self.CurrentIndex`)))
  (for _index (range 2)
    (set `self.CurrentIndex` _index)
    (`GameplayStatics.CreatePlayer` -1)
    (bind _returnvalue_2 (`|SpawnActorFromClass` "/Game/Blueprints/Framework/BP_Character.BP_Character_C" (`KismetMathLibrary.MakeTransform` (`KismetMathLibrary.MakeVector` 0.0 (* (`self.CurrentIndex`) 200.0))) "Undefined" "OverrideRootScale" null null))
    (`Controller.Possess` _returnvalue _returnvalue_2)
    (`PlayerController.SetViewTargetWithBlend` _returnvalue (`self.CameraRef`) 0.0 "VTBlend_Linear" 0.0 false)))

(fn `StartGame`
  (returns (Return :type Boolean))
  (`KismetSystemLibrary.PrintString` "Start Game ")
  (set `self.CurrentGameState` "NewEnumerator4")
  (return false))

(fn `UserConstructionScript`)