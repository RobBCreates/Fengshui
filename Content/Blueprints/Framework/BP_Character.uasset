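; Player character pawn for grid-based movement with 2D flipbook sprites, using per-PlayerID animation and sound sets.
; Directional input asks BP_GridManager for the next point, then timelines lerp position and PaperSprite scale while the game-mode state permits.
; Blocked moves push the occupying interactable through interface messages and play push flipbooks.
; Interact traces the facing point, and holding it makes movement pull that object along.
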(event `self.ReceiveBeginPlay`
  (`self.Init`))

(event `Move`
  (params (Direction :type "Vector Structure"))
  (bind _returnvalue (* (`self.CurrentDirection`) 100.0))
  (bind _currentstate (message `/Game/Blueprints/Interfaces/BPI_GameMode.GetGameState` (`GameplayStatics.GetGameMode`)))
  (if (`|EnumEquality` _currentstate "NewEnumerator1")
    (set `self.CurrentDirection` Direction)
    (set `self.StartLocation` (`self.K2_GetActorLocation`))
    (bind (_isspaceavailable _newgridlocation) (`/Game/Blueprints/Grid/BP_GridManager.IsNodeAvailable` (`self.GridManager`) (`self.CurrentGridPoint`) _returnvalue))
    (if _isspaceavailable
      (`/Game/Blueprints/Grid/BP_GridManager.UpdateLocation` (`self.GridManager`) (`self.CurrentGridPoint`) _newgridlocation)
      (`self.MoveAnimation`)
      (`GameplayStatics.PlaySoundAtLocation` (`self.SoundMove`) (`self.K2_GetActorLocation`) (struct) 1.0 1.0 0.0 null null null)
      (set `self.NewPosition` (+ (`self.StartLocation`) _returnvalue))
      (set `self.bMoving` true)
      (`|ExecutionSequence`
        (:`then_0`
          (bind (_direction _deleta) (`Timeline|MoveTimeline` :!via `PlayFromStart`)
            (:`Update`
              (`self.K2_SetActorLocation` (`KismetMathLibrary.VLerp` (`self.StartLocation`) (`self.NewPosition`) _deleta)))
            (:`Finished`
              (set `self.bMoving` false)
              (set `self.CurrentGridPoint` _newgridlocation)
              (`PaperFlipbookComponent.SetFlipbook` (`self.Sprite`) (select `/Game/Blueprints/Framework/EMoveDirection` (`self.Direction`) :`NewEnumerator0` (`self.FB_IdleBack`) :`NewEnumerator4` (`self.FB_IdleFront`) :`NewEnumerator1` (`self.FB_IdleSide`) :`NewEnumerator2` (`self.FB_IdleSide`)))
              (`GameplayStatics.PlaySoundAtLocation` (`self.SoundLandWood`) (`self.K2_GetActorLocation`) (struct) 1.0 1.0 0.0 null null null))))
        (:`then_1`
          (bind (_direction_2 _newtrack_0) (`Timeline|LerpShadow` :!via `PlayFromStart`)
            (:`Update`
              (`SceneComponent.SetWorldScale3D` (`self.PaperSprite`) (`KismetMathLibrary.VLerp` (0.15 0.15 0.15) (0.2 0.2 0.2) _newtrack_0))))))
      (else
        (`self.PushObject` _newgridlocation)))))

(event `Pull`
  (params (Direction :type "Vector Structure"))
  (`self.Move` Direction)
  (bind _interactingobject (`self.InteractingObject`)
    (:`then`
      (message `/Game/Blueprints/Interactable/BPI_Interactable.MoveInteractable` _interactingobject Direction))
    (:`else`)))

(event `InputAction|Forward`
  (params (Key :type "Key Structure"))
  (:`Pressed`
    (if (not (`self.bMoving`))
      (set `self.Direction` "NewEnumerator0")
      (if (`self.CanPull`)
        (`self.Pull` (1.0 0.0 0.0))
        (else
          (`self.Move` (1.0 0.0 0.0)))))))

(event `InputAction|Backward`
  (params (Key :type "Key Structure"))
  (:`Pressed`
    (if (not (`self.bMoving`))
      (set `self.Direction` "NewEnumerator4")
      (if (`self.CanPull`)
        (`self.Pull` (-1.0 0.0 0.0))
        (else
          (`self.Move` (-1.0 0.0 0.0)))))))

(event `InputAction|Left`
  (params (Key :type "Key Structure"))
  (:`Pressed`
    (if (not (`self.bMoving`))
      (set `self.Direction` "NewEnumerator1")
      (if (`self.CanPull`)
        (`self.Pull` (0.0 -1.0 0.0))
        (else
          (`self.Move` (0.0 -1.0 0.0)))))))

(event `InputAction|Right`
  (params (Key :type "Key Structure"))
  (:`Pressed`
    (if (not (`self.bMoving`))
      (set `self.Direction` "NewEnumerator2")
      (if (`self.CanPull`)
        (`self.Pull` (0.0 1.0 0.0))
        (else
          (`self.Move` (0.0 1.0 0.0)))))))

(event `InputAction|Interact`
  (params (Key :type "Key Structure"))
  (:`Pressed`
    (set `self.bIsInteracting` true)
    (bind (_gridpoint _actorongridpoint) (`/Game/Blueprints/Interactable/SceneComp_TracePoint.TraceForwardInteract` (`self.SceneComp_TracePoint`) (`self.CurrentDirection`) (`self.CurrentGridPoint`)))
    (`/Engine/EditorBlueprintResources/StandardMacros.IsValid` _actorongridpoint
      (:`Is Valid`
        (message `/Game/Blueprints/Interactable/BPI_Interactable.Interact` _actorongridpoint)
        (set `self.InteractingObject` _actorongridpoint))
      (:`Is Not Valid`
        (`KismetSystemLibrary.PrintString` "No actor to interact with"))))
  (:`Released`
    (set `self.bIsInteracting` true)
    (set `self.InteractingObject` null)))

(fn `CanPull`
  (returns (CanPull :type Boolean))
  (return (and (`self.bIsInteracting`) (`KismetSystemLibrary.IsValid` (`self.InteractingObject`)))))

(fn `Init`
  (set `self.bMoving` false)
  (set `self.Direction` "NewEnumerator0")
  (`self.ResetIdle`)
  (`TimelineComponent.SetPlayRate` (`self.MoveTimeline`) 3.0)
  (`TimelineComponent.SetPlayRate` (`self.LerpShadow`) 3.0)
  (`|ExecutionSequence`
    (:`then_0`
      (bind _returnvalue (`GameplayStatics.GetActorOfClass` "/Game/Blueprints/Grid/BP_GridManager.BP_GridManager_C"))
      (bind _output_get (set `self.GridManager` _returnvalue))
      (`/Engine/EditorBlueprintResources/StandardMacros.IsValid` _output_get
        (:`Is Valid`
          (`/Game/Blueprints/Grid/BP_GridManager.SnapToGrid` (`self.GridManager`) self)
          (`self.SetupGridReference`))))
    (:`then_1`
      (bind _returnvalue_2 (`GameplayStatics.GetActorOfClass` "/Game/Blueprints/Framework/BP_Camera.BP_Camera_C"))
      (set `self.CameraRef` _returnvalue_2))))

(fn `MoveAnimation`
  (bind (_currentdirection_x _currentdirection_y) (`KismetMathLibrary.BreakVector` (`self.CurrentDirection`)))
  (bind _currentdirection_x_2 (`KismetMathLibrary.BreakVector` (`self.CurrentDirection`)))
  (bind _currentdirection_x_3 (`KismetMathLibrary.BreakVector` (`self.CurrentDirection`)))
  (bind (_returnvalue_x _returnvalue_y _returnvalue_z) (`KismetMathLibrary.BreakVector` (`SceneComponent.K2_GetComponentScale` (`self.Sprite`))))
  (bind (_returnvalue_x_2 _returnvalue_y_2 _returnvalue_z_2) (`KismetMathLibrary.BreakVector` (`SceneComponent.K2_GetComponentScale` (`self.Sprite`))))
  (if (!= _currentdirection_x_2 0.0)
    (`SceneComponent.SetWorldScale3D` (`self.Sprite`) (`KismetMathLibrary.MakeVector` (* (`KismetMathLibrary.Abs` _returnvalue_x_2) _currentdirection_x_3) _returnvalue_y_2 _returnvalue_z_2))
    (`PaperFlipbookComponent.SetFlipbook` (`self.Sprite`) (select `bool` (`|EnumEquality` (`self.Direction`) "NewEnumerator0") :`false` (`self.FB_RunBack`) :`true` (`self.FB_RunForward`)))
    (else
      (`SceneComponent.SetWorldScale3D` (`self.Sprite`) (`KismetMathLibrary.MakeVector` (* (`KismetMathLibrary.Abs` _returnvalue_x) _currentdirection_y) _returnvalue_y _returnvalue_z))
      (`PaperFlipbookComponent.SetFlipbook` (`self.Sprite`) (`self.FB_RunSide`)))))

(fn `PushObject`
  (params (GridPointOfInteractable :type "/Game/Blueprints/Grid/BP_GridPoint Object Reference"))
  (bind (_currentdirection_x _currentdirection_y) (`KismetMathLibrary.BreakVector` (`self.CurrentDirection`)))
  (bind _fb_pushside (`self.FB_PushSide`))
  (bind _currentdirection_x_2 (`KismetMathLibrary.BreakVector` (`self.CurrentDirection`)))
  (bind _currentdirection_x_3 (`KismetMathLibrary.BreakVector` (`self.CurrentDirection`)))
  (bind (_returnvalue_x _returnvalue_y _returnvalue_z) (`KismetMathLibrary.BreakVector` (`SceneComponent.K2_GetComponentScale` (`self.Sprite`))))
  (bind (_returnvalue_x_2 _returnvalue_y_2 _returnvalue_z_2) (`KismetMathLibrary.BreakVector` (`SceneComponent.K2_GetComponentScale` (`self.Sprite`))))
  (bind _returnvalue (select `bool` (`|EnumEquality` (`self.Direction`) "NewEnumerator0") :`false` (`self.FB_PushForward`) :`true` (`self.FB_PushBack`)))
  (`/Engine/EditorBlueprintResources/StandardMacros.IsValid` GridPointOfInteractable
    (:`Is Valid`
      (bind _asbp_interactable_base (cast `/Game/Blueprints/Interactable/BP_InteractableBase` (`/Game/Blueprints/Grid/BP_GridPoint.ActorOnGridPoint` GridPointOfInteractable)))
      (message `/Game/Blueprints/Interactable/BPI_Interactable.MoveInteractable` _asbp_interactable_base (`self.CurrentDirection`))
      (if (!= _currentdirection_x_2 0.0)
        (`SceneComponent.SetWorldScale3D` (`self.Sprite`) (`KismetMathLibrary.MakeVector` (* (`KismetMathLibrary.Abs` _returnvalue_x_2) _currentdirection_x_3) _returnvalue_y_2 _returnvalue_z_2))
        (`PaperFlipbookComponent.SetFlipbook` (`self.Sprite`) _returnvalue)
        (`KismetSystemLibrary.K2_SetTimer` null "ResetIdle" (`PaperFlipbook.GetTotalDuration` _returnvalue))
        (else
          (`SceneComponent.SetWorldScale3D` (`self.Sprite`) (`KismetMathLibrary.MakeVector` (* (`KismetMathLibrary.Abs` _returnvalue_x) _currentdirection_y) _returnvalue_y _returnvalue_z))
          (`PaperFlipbookComponent.SetFlipbook` (`self.Sprite`) _fb_pushside)
          (`KismetSystemLibrary.K2_SetTimer` null "ResetIdle" (`PaperFlipbook.GetTotalDuration` _fb_pushside)))))))

(fn `ResetIdle`
  (if (not (`self.bMoving`))
    (`PaperFlipbookComponent.SetFlipbook` (`self.Sprite`) (select `/Game/Blueprints/Framework/EMoveDirection` (`self.Direction`) :`NewEnumerator0` (`self.FB_IdleBack`) :`NewEnumerator4` (`self.FB_IdleFront`) :`NewEnumerator1` (`self.FB_IdleSide`) :`NewEnumerator2` (`self.FB_IdleSide`)))))

(fn `SetupGridReference`
  (bind _gridpoint (`/Game/Blueprints/Interactable/SceneComp_TracePoint.TraceDownForGridPoint` (`self.SceneComp_TracePoint`)))
  (set `self.CurrentGridPoint` _gridpoint))

(fn `UserConstructionScript`
  (switch `int` (`self.PlayerID`)
    (:`0`
      (set `self.FB_RunForward` "/Game/Assets/Flipbooks/Char1/player-backMove.player-backMove")
      (set `self.FB_RunBack` "/Game/Assets/Flipbooks/Char1/player-frontMove.player-frontMove")
      (set `self.FB_RunSide` "/Game/Assets/Flipbooks/Char1/player-sideMove.player-sideMove")
      (set `self.FB_IdleBack` "/Game/Assets/Flipbooks/Char1/player-backIdle.player-backIdle")
      (set `self.FB_IdleFront` "/Game/Assets/Flipbooks/Char1/player-frontIdle.player-frontIdle")
      (set `self.FB_IdleSide` "/Game/Assets/Flipbooks/Char1/player-sideIdle.player-sideIdle")
      (set `self.FB_PushForward` "/Game/Assets/Flipbooks/Char1/player-frontPush.player-frontPush")
      (set `self.FB_PushBack` "/Game/Assets/Flipbooks/Char1/player-backPush.player-backPush")
      (set `self.FB_PushSide` "/Game/Assets/Flipbooks/Char1/player-sidePush.player-sidePush")
      (set `self.SoundMove` "/Game/Audio/Move/MOVE_Character1_01_Cue.MOVE_Character1_01_Cue")
      (set `self.SoundLandWood` "/Game/Audio/Footsteps/Character_1/FTSTP_Character1_Wood_01_Cue.FTSTP_Character1_Wood_01_Cue")
      (set `self.SoundVO` "/Game/Audio/VO/VO_Keith_01_Cue.VO_Keith_01_Cue"))
    (:`1`
      (set `self.FB_RunForward` "/Game/Assets/Flipbooks/Char2/player2-backMove.player2-backMove")
      (set `self.FB_RunBack` "/Game/Assets/Flipbooks/Char2/player2-frontMove.player2-frontMove")
      (set `self.FB_RunSide` "/Game/Assets/Flipbooks/Char2/player2-sideMove.player2-sideMove")
      (set `self.FB_IdleBack` "/Game/Assets/Flipbooks/Char2/player2-backIdle.player2-backIdle")
      (set `self.FB_IdleFront` "/Game/Assets/Flipbooks/Char2/player2-frontIdle.player2-frontIdle")
      (set `self.FB_IdleSide` "/Game/Assets/Flipbooks/Char2/player2-sideIdle.player2-sideIdle")
      (set `self.FB_PushForward` "/Game/Assets/Flipbooks/Char2/player2-frontPush.player2-frontPush")
      (set `self.FB_PushBack` "/Game/Assets/Flipbooks/Char2/player2-backPush.player2-backPush")
      (set `self.FB_PushSide` "/Game/Assets/Flipbooks/Char2/player2-sidePush.player2-sidePush")
      (set `self.SoundLandWood` "/Game/Audio/Move/MOVE_Character2_01_Cue.MOVE_Character2_01_Cue")
      (set `self.SoundLandWood` "/Game/Audio/Footsteps/Character_2/FTSTP_Character2_Wood_01_Cue.FTSTP_Character2_Wood_01_Cue")
      (set `self.SoundVO` "/Game/Audio/VO/VO_Carol_05_Cue.VO_Carol_05_Cue"))))