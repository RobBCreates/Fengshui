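; BP_GridManager manages a grid of BP_GridPoint actors, snapping actors to it and tracking which points are available for movement.
; AllGridPoints lazily finds and caches every grid point, and the construction script snaps the manager itself to GridSize.
; IsNodeAvailable matches a grid-snapped offset from the current point to another point within a tolerance and returns its availability.
; UpdateLocation frees the old point and marks the new one occupied.
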(event `self.ReceiveBeginPlay`)

(fn `All Grid Points`
  (returns (AllGridPoints :type "Array of /Game/Blueprints/Grid/BP_GridPoint Object Reference"))
  (if (> (`KismetArrayLibrary.Array_Length` (`self.GridPoints`)) 0)
    (return (`self.GridPoints`))
    (else
      (bind _outactors (`GameplayStatics.GetAllActorsOfClass` "/Game/Blueprints/Grid/BP_GridPoint.BP_GridPoint_C"))
      (bind _output_get (set `self.GridPoints` _outactors))
      (return _output_get))))

(fn `IsNodeAvailable`
  (params (CurrentGridPoint :type "/Game/Blueprints/Grid/BP_GridPoint Object Reference") (DistanceToTravel :type "Vector Structure"))
  (returns (IsSpaceAvailable :type Boolean) (NewGridLocation :type "/Game/Blueprints/Grid/BP_GridPoint Object Reference"))
  (locals (L_bIsSpaceAvailable :type Boolean :default false) (L_NewGridLocation :type "/Game/Blueprints/Grid/BP_GridPoint Object Reference"))
  (for _array_element (`self.All Grid Points`)
    (if (== (`self.K2_GetActorLocation` _array_element) (+ (`self.K2_GetActorLocation` CurrentGridPoint) (`KismetMathLibrary.Vector_SnappedToGrid` DistanceToTravel (`self.GridSize`))) :`ErrorTolerance` 10.0)
      (set `local.L_NewGridLocation` _array_element)
      (set `local.L_bIsSpaceAvailable` (`/Game/Blueprints/Grid/BP_GridPoint.bIsAvailable` _array_element))
      (break)
      (else
        (set `local.L_bIsSpaceAvailable` true))))
  (`/Engine/EditorBlueprintResources/StandardMacros.IsValid` (`local.L_NewGridLocation`)
    (:`Is Valid`
      (return (`local.L_bIsSpaceAvailable`) (`local.L_NewGridLocation`)))
    (:`Is Not Valid`
      (`KismetSystemLibrary.PrintString` "Invalid move location")
      (return false null))))

(fn `SnapToGrid`
  (params (ActorRef :type "Actor Object Reference"))
  (`self.K2_SetActorLocation` ActorRef (`KismetMathLibrary.Vector_SnappedToGrid` (`self.K2_GetActorLocation` ActorRef) (`self.GridSize`)) false false))

(fn `UpdateLocation`
  (params (CurrentLocation :type "/Game/Blueprints/Grid/BP_GridPoint Object Reference") (NewLocation :type "/Game/Blueprints/Grid/BP_GridPoint Object Reference"))
  (if (and (`KismetSystemLibrary.IsValid` CurrentLocation) (`KismetSystemLibrary.IsValid` NewLocation))
    (set `/Game/Blueprints/Grid/BP_GridPoint.bIsAvailable` true CurrentLocation)
    (set `/Game/Blueprints/Grid/BP_GridPoint.bIsAvailable` false NewLocation)))

(fn `UserConstructionScript`
  (`self.K2_SetActorLocation` (`KismetMathLibrary.Vector_SnappedToGrid` (`self.K2_GetActorLocation`) (`self.GridSize`))))