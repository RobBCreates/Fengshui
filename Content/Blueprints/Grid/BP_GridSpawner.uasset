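; BP_GridSpawner is a grid actor with a Box component, apparently intended to spawn grid points within its bounds.
; On BeginPlay it finds the BP_GridManager actor and caches the reference.
; SpawnGridPoints loops over the box's scaled X extent divided by the manager's GridSize, but the loop body is empty and nothing in the file calls it.
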(event `self.ReceiveBeginPlay`
  (bind _returnvalue (`GameplayStatics.GetActorOfClass` "/Game/Blueprints/Grid/BP_GridManager.BP_GridManager_C"))
  (set `self.GridManagerRef` _returnvalue))

(fn `SpawnGridPoints`
  (for _ (range (+ (`KismetMathLibrary.FTrunc` (/ (.x (`BoxComponent.GetScaledBoxExtent` (`self.Box`))) (`/Game/Blueprints/Grid/BP_GridManager.GridSize` (`self.GridManagerRef`)))) 1))
    _))

(fn `UserConstructionScript`)