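; Audio manager Blueprint that handles switching between menu music and in-game music.
; On BeginPlay it fades in the menu track, and EnterGameMusic quickly fades that out while fading in the game track.
; An intro-sting path that would schedule PlayLevelMusic by timer is disconnected, and PlayLevelMusic is empty.
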(event `self.ReceiveBeginPlay`
  (`AudioComponent.FadeIn` (`self.MenuMusic`) 2.0 1.0 0.0 "Linear"))

(fn `EnterGameMusic`
  (`AudioComponent.FadeOut` (`self.MenuMusic`) 0.5 0.0 "Linear")
  (`AudioComponent.FadeIn` (`self.GameMusic`) 0.1 1.0 0.0 "Linear"))

(fn `PlayLevelMusic`)

(fn `UserConstructionScript`)