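; Interactable radio actor that cycles through two music channels and silence each time the player interacts with it.
; Its audio component starts playing muted on BeginPlay, so switching only changes volume and channel rather than restarting playback.
; Each interaction plays a retune sound, then either flips the SwitchChannel bool parameter at full volume or mutes the audio and resets the cycle.
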(event `self.ReceiveBeginPlay`
  (bind _audio (`self.Audio`))
  (`parent.ReceiveBeginPlay`)
  (`ActorComponent.Activate` _audio false)
  (`AudioComponent.Play` _audio 0.0)
  (`AudioComponent.SetVolumeMultiplier` (`self.Audio`) 0.0))

(event `self.ReceiveTick`
  (params (DeltaSeconds :type "Float (single-precision)")))

(fn `Interact`
  (returns (Return :type Boolean))
  (`AudioComponent.Play` (`self.RetuneSound`) 0.0)
  (switch `int` (`self.MusicChoice`)
    (:`0`
      (set `self.CurrentAudio` (not (`self.CurrentAudio`)) :!label _label)
      (`AudioComponent.SetBoolParameter` (`self.Audio`) "SwitchChannel" (`self.CurrentAudio`))
      (`AudioComponent.SetVolumeMultiplier` (`self.Audio`) 1.0)
      (`/Engine/EditorBlueprintResources/StandardMacros.IncrementInt` (`self.MusicChoice`)
        (:`  `
          _)))
    (:`1`
      (goto _label))
    (:`2`
      (`AudioComponent.SetVolumeMultiplier` (`self.Audio`) 0.0)
      (set `self.MusicChoice` 0)))
  (return false))

(fn `UserConstructionScript`
  (`parent.UserConstructionScript`))