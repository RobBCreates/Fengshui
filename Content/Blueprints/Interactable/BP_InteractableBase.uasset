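; Base actor for grid-based interactables, which snaps to BP_GridManager's grid on BeginPlay and can be moved one 100-unit step at a time.
; A move asks the grid manager whether the target is free, updates its location there, then plays a sound and lerps the actor across on a timeline.
; Child trace-point components trace down to set the grid location, which supports only one point.
; Interact only prints, and PushObject is empty.
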(event `self.ReceiveBeginPlay`
  (bind _returnvalue (`GameplayStatics.GetActorOfClass` "/Game/Blueprints/Grid/BP_GridManager.BP_GridManager_C"))
  (bind _output_get (set `self.GridManagerRef` _returnvalue))
  (`/Game/Blueprints/Grid/BP_GridManager.SnapToGrid` _output_get self)
  (`self.OccupyGridPoints`))

(event `MoveDirection`
  (params (CurrentDirection :type "Vector Structure"))
  (bind _returnvalue (* (`self.CurrentDirection`) 100.0))
  (set `self.CurrentDirection` CurrentDirection)
  (if (not (`self.bMoving`))
    (set `self.StartLocation` (`self.K2_GetActorLocation`))
    (bind (_isspaceavailable _newgridlocation) (`/Game/Blueprints/Grid/BP_GridManager.IsNodeAvailable` (`self.GridManagerRef`) (`self.GridPointLocation`) _returnvalue))
    (if _isspaceavailable
      (`/Game/Blueprints/Grid/BP_GridManager.UpdateLocation` (`self.GridManagerRef`) (`self.GridPointLocation`) _newgridlocation)
      (set `self.NewPosition` (+ (`self.StartLocation`) _returnvalue))
      (set `self.bMoving` true)
      (`GameplayStatics.PlaySoundAtLocation` (`self.ObjectSoundType`) (`self.K2_GetActorLocation`) (struct) 1.0 1.0 0.0 null null null)
      (bind (_direction _deleta) (`Timeline|Timeline_0` :!via `PlayFromStart`)
        (:`Update`
          (`self.K2_SetActorLocation` (`KismetMathLibrary.VLerp` (`self.StartLocation`) (`self.NewPosition`) _deleta)))
        (:`Finished`
          (set `self.bMoving` false)
          (`self.OccupyGridPoints`))))))

(fn `Get All Trace Components`
  (returns (AllTracePoints :type "Array of /Game/Blueprints/Interactable/SceneComp_TracePoint Object Reference"))
  (locals (L_AllTracePoints :type "Array of /Game/Blueprints/Interactable/SceneComp_TracePoint Object Reference"))
  (for _array_element (`SceneComponent.GetChildrenComponents` (`self.DefaultSceneRoot`) true)
    (bind _asscene_comp_trace_point (cast `/Game/Blueprints/Interactable/SceneComp_TracePoint` _array_element))
    (`KismetArrayLibrary.Array_AddUnique` (`local.L_AllTracePoints`) _asscene_comp_trace_point))
  (return (`local.L_AllTracePoints`)))

(fn `Interact`
  (returns (Return :type Boolean))
  (`KismetSystemLibrary.PrintString` (`KismetStringLibrary.Concat_StrStr` (`KismetSystemLibrary.GetDisplayName` self) " Interact") true true (struct :`G` 0.66 :`B` 1.0 :`A` 1.0) 5.0)
  (return false))

(fn `MoveInteractable`
  (params (Direction :type "Vector Structure"))
  (returns (CanMove :type Boolean))
  (`self.MoveDirection` Direction)
  (return false))

(fn `OccupyGridPoints`
  ;[1 1 1] Only works for one trace point
  (for _array_element (`self.Get All Trace Components`)
    (bind _gridpoint (`/Game/Blueprints/Interactable/SceneComp_TracePoint.TraceDownForGridPoint` _array_element))
    (set `self.GridPointLocation` _gridpoint)))

(fn `PushObject`
  (params (GridPointOfInteractable :type "/Game/Blueprints/Grid/BP_GridPoint Object Reference")))

(fn `UserConstructionScript`)