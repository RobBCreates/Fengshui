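; An interactable lamp that the player toggles on and off.
; On BeginPlay it stores the point light's starting intensity, switches the light off, and puts a dynamic instance of a flat yellow material on one mesh slot.
; Interact flips the on state, restoring or zeroing light intensity and emissive strength and playing the matching switch sound in 2D, then returns false.
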(event `self.ReceiveBeginPlay`
  (bind _staticmesh (`self.StaticMesh`))
  (`parent.ReceiveBeginPlay`)
  (set `self.InitIntensity` (`LightComponentBase.Intensity` (`self.PointLight`)))
  (`LightComponent.SetIntensity` (`self.PointLight`) 0.0)
  (bind _returnvalue (`PrimitiveComponent.CreateDynamicMaterialInstance` _staticmesh 3 "/Game/Assets/Materials/M_FlatYellow.M_FlatYellow" "None"))
  (bind _output_get (set `self.LampMaterial` _returnvalue))
  (`PrimitiveComponent.SetMaterial` _staticmesh 3 _output_get))

(fn `Interact`
  (returns (Return :type Boolean))
  (bind _output_get (set `self.bIsOn` (not (`self.bIsOn`))))
  (if _output_get
    (`LightComponent.SetIntensity` (`self.PointLight`) (`self.InitIntensity`))
    (`MaterialInstanceDynamic.SetScalarParameterValue` (`self.LampMaterial`) "EmissiveStrength" 10.0)
    (`GameplayStatics.PlaySound2D` "/Game/Audio/Lamp/OBJ_Lamp_SwitchOn.OBJ_Lamp_SwitchOn" 1.0 1.0 0.0 null null)
    (else
      (`LightComponent.SetIntensity` (`self.PointLight`) 0.0)
      (`MaterialInstanceDynamic.SetScalarParameterValue` (`self.LampMaterial`) "EmissiveStrength" 0.0)
      (`GameplayStatics.PlaySound2D` "/Game/Audio/Lamp/OBJ_Lamp_SwitchOff.OBJ_Lamp_SwitchOff" 1.0 1.0 0.0 null null)))
  (return false))

(fn `UserConstructionScript`
  (`parent.UserConstructionScript`))