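; Scene component that finds grid points from its world location and marks them as occupied by its owning actor.
; One function line-traces vertically through the component, the other traces a short horizontal distance along a supplied last direction, both against WorldDynamic objects with debug drawing on.
; A hit BP_GridPoint is flagged unavailable, given the owner as its occupant and returned; neither function releases a previously claimed point.
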(fn `TraceDownForGridPoint`
  (returns (GridPoint :type "/Game/Blueprints/Grid/BP_GridPoint Object Reference"))
  (bind (_outhit _returnvalue) (`KismetSystemLibrary.LineTraceSingleForObjects` :`Start` (+ (`self.K2_GetComponentLocation`) (0.0 0.0 100.0)) :`End` (- (`self.K2_GetComponentLocation`) (0.0 0.0 100.0)) :`ObjectTypes` (`|MakeArray` "ObjectTypeQuery2" :!type "EObjectTypeQuery Enum") :`DrawDebugType` "ForDuration" :`bIgnoreSelf` false))
  (if _returnvalue
    (bind _asbp_grid_point (cast `/Game/Blueprints/Grid/BP_GridPoint` (`.HitActor` (`GameplayStatics.BreakHitResult` _outhit))))
    (set `/Game/Blueprints/Grid/BP_GridPoint.bIsAvailable` false _asbp_grid_point)
    (set `/Game/Blueprints/Grid/BP_GridPoint.ActorOnGridPoint` (`self.GetOwner`) _asbp_grid_point)
    (return _asbp_grid_point)))

(fn `TraceForwardForGridPoint`
  (params (LastDirection :type "Vector Structure"))
  (returns (GridPoint :type "/Game/Blueprints/Grid/BP_GridPoint Object Reference"))
  (bind (_outhit _returnvalue) (`KismetSystemLibrary.LineTraceSingleForObjects` :`Start` (+ (`self.K2_GetComponentLocation`) (0.0 0.0 0.0)) :`End` (+ (`self.K2_GetComponentLocation`) (* LastDirection (50.0 50.0 0.0))) :`ObjectTypes` (`|MakeArray` "ObjectTypeQuery2" :!type "EObjectTypeQuery Enum") :`DrawDebugType` "ForDuration" :`bIgnoreSelf` false))
  (if _returnvalue
    (bind _asbp_grid_point (cast `/Game/Blueprints/Grid/BP_GridPoint` (`.HitActor` (`GameplayStatics.BreakHitResult` _outhit))))
    (set `/Game/Blueprints/Grid/BP_GridPoint.bIsAvailable` false _asbp_grid_point)
    (set `/Game/Blueprints/Grid/BP_GridPoint.ActorOnGridPoint` (`self.GetOwner`) _asbp_grid_point)
    (return _asbp_grid_point)))